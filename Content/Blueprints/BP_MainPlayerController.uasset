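; BP_MainPlayerController is a player controller that replaces the Hand mouse cursor with a custom widget.
; On BeginPlay it creates the cursor widget, assigns it and prints a debug "Hello".
; Unconnected leftover nodes sketch click handling through HandleClick and cursor-trace selection that deselects the previous BP_ClickableActor, but none of them run.
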(event EventBeginPlay
  (bind _returnvalue (UserInterface|CreateWidget "/Game/Blueprints/MouseCursorWidget.MouseCursorWidget_C"))
  (Class|PlayerController|SetMouseCursorWidget "Hand" _returnvalue)
  (Development|PrintString "Hello"))

(event Input|ActionEvents|InputActionLeftActionButton
  (params (Key :type Key%20Structure)))

(fn ConstructionScript)