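; Test actor that plots a sine wave in the world by leaving a trail of spawned BP_SineSphereTest actors.
; Each Tick offsets its Sphere along relative X via a sine math expression, drifts the actor along world Y, and spawns at the Sphere's location.
; SinA and SinB grow every frame, SinA compounding, and are printed on screen.
; Older timeline and sphere-trace experiments remain disconnected.
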(event Custom|DrawDebugSphere
  ;[1 1 1] DrawDebug
  (Game|SpawnActorfromClass "/Game/Blueprints/TestStuff/BP_SineSphereTest.BP_SineSphereTest_C" (Math|Transform|MakeTransform (Transformation|GetWorldLocation (Variables|Default|GetSphere)) "0, 0, 0" "1,1,1") "AlwaysSpawn" 0 0))

(event Custom|AddMovementOnRightAxis
  ;[1 1 1] AddMovement
  (Transformation|AddActorWorldOffset (Math|Vector|MakeVector 0.0 (* (Utilities|Time|GetWorldDeltaSeconds) 1e+01) 0.0)))

(event Custom|SetSphereLocation
  ;[1 1 1] SetSphereLocation
  (Transformation|SetRelativeLocation (Variables|Default|GetSphere) (Math|Vector|MakeVector (|((sin((x*{D2F8CD5F-4087-C528-4B5C-F6A2122921CB})))*{9568E73A-454F-71DF-ABAB-779B25A56587}) 1.0) 0.0 0.0) false false))

(event Custom|ChangeABValues
  (bind _output_get (Variables|Default|SetSinA (+ (/ (Utilities|Time|GetWorldDeltaSeconds) 2.0) (Variables|Default|GetSinA) (/ (Variables|Default|GetSinA) 5.0))))
  (bind _output_get_2 (Variables|Default|SetSinB (+ (* (Utilities|Time|GetWorldDeltaSeconds) 2.0) (Variables|Default|GetSinB))))
  (Development|PrintString (Utilities|String|ToString(Text) (Utilities|Text|FormatText "A: {0} 
B: {1}" _output_get _output_get_2)) true true "(R=0.000000,G=0.660000,B=1.000000,A=1.000000)" (Utilities|Time|GetWorldDeltaSeconds)))

(event EventTick
  (params (DeltaSeconds :type Float%20%28single-precision%29))
  (Utilities|FlowControl|Sequence
    (:then_0
      (CallFunction|SetSphereLocation))
    (:then_1
      (CallFunction|AddMovementonRightAxis))
    (:then_2
      (CallFunction|ChangeABValues))
    (:then_3
      (CallFunction|DrawDebugSphere))))

(fn ConstructionScript)