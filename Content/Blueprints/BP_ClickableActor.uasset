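; BP_ClickableActor is an actor that can be selected by clicking, showing its state through the material on its Sphere component.
; On BeginPlay it binds its own handlers to its OnSelected and OnDeselected dispatchers.
; A click prints a debug message and calls OnSelected, while the DeselectActor function calls OnDeselected.
; The handlers set IsSelected and swap the Sphere between selected and basic materials.
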(event Custom|OnSelected_Event
  (Variables|Default|SetIsSelected true)
  (Rendering|Material|SetMaterial (Variables|Default|GetSphere) 0 "/Game/Materials/M_SelectedActor.M_SelectedActor"))

(event Custom|OnDeselected_Event
  (Variables|Default|SetIsSelected false)
  (Rendering|Material|SetMaterial (Variables|Default|GetSphere) 0 "/Engine/BasicShapes/BasicShapeMaterial.BasicShapeMaterial"))

(event EventBeginPlay
  (EventDispatchers|BindEventtoOnSelected (EventDispatchers|CreateEvent :!event Custom|OnSelected_Event))
  (EventDispatchers|BindEventtoOnDeselected (EventDispatchers|CreateEvent :!event Custom|OnDeselected_Event)))

(event MouseInput|EventActorOnClicked
  (params (ButtonPressed :type Key%20Structure))
  (Development|PrintString "I am Clicked")
  (Default|CallOnSelected))

(fn ConstructionScript)

(fn DeselectActor
  (Default|CallOnDeselected))